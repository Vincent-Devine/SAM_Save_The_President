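; Trigger volume that shows a tutorial popup while the player stands inside it.
; On BeginPlay it creates a BP_TutorialWidget for the first player controller, fills its header and description from the WidgetHeader and WidgetDescription variables, and adds it hidden to the player screen.
; Box overlap begin and end events toggle the widget's visibility for actors tagged "Player".
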(event `self.ReceiveBeginPlay`
  (bind _returnvalue (`|CreateWidget` "/Game/Blueprints/BP_TutorialWidget.BP_TutorialWidget_C" (`GameplayStatics.GetPlayerController` 0)))
  (bind _output_get (set `self.TutorialWidgetRef` _returnvalue))
  (`TextBlock.SetText` (`/Game/Blueprints/BP_TutorialWidget.Header` _output_get) (`self.WidgetHeader`))
  (`TextBlock.SetText` (`/Game/Blueprints/BP_TutorialWidget.Description` _output_get) (`self.WidgetDescription`))
  (`Widget.SetVisibility` _returnvalue "Hidden")
  (`UserWidget.AddToPlayerScreen` _returnvalue 0))

(event `self.Box.OnComponentBeginOverlap`
  (params (OverlappedComponent :type "PrimitiveComponent Object Reference") (OtherActor :type "Actor Object Reference") (OtherComp :type "PrimitiveComponent Object Reference") (OtherBodyIndex :type Integer) (bFromSweep :type Boolean) (SweepResult :type "HitResult Structure (by ref)"))
  (if (`self.ActorHasTag` OtherActor "Player")
    (`Widget.SetVisibility` (`self.TutorialWidgetRef`) "Visible")))

(event `self.Box.OnComponentEndOverlap`
  (params (OverlappedComponent :type "PrimitiveComponent Object Reference") (OtherActor :type "Actor Object Reference") (OtherComp :type "PrimitiveComponent Object Reference") (OtherBodyIndex :type Integer))
  (if (`self.ActorHasTag` OtherActor "Player")
    (`Widget.SetVisibility` (`self.TutorialWidgetRef`) "Hidden")))

(fn `UserConstructionScript`)